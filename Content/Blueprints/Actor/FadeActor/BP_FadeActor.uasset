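; BP_FadeActor is a mesh actor that fades out and back in through a material "Fade" parameter.
; The construction script caches original materials and builds dynamic instances from FadeMaterialInsts.
; FadeOut swaps in those instances and plays a timeline driving Fade; Fadein reverses it.
; When the timeline finishes with Fade at one or above, original materials are restored; Visibility collision toggles are left unwired.
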(event EventBeginPlay)

(event EventFadeOut
  (CallFunction|SetMaterialtoDynamicInsts)
  (bind _fade (Timeline|FadeTimeLine Play)
    (:Update
      (for _array_element (Variables|Default|GetDynamicMaterialnsts)
        (Rendering|Material|SetScalarParameterValue _array_element "Fade" _fade :!class /Script/Engine.MaterialInstanceDynamic)))
    (:Finished
      (CallFunction|FadeFinishes _fade))))

(event EventFadein
  (bind _fade (Timeline|FadeTimeLine Reverse)
    (:Update
      (for _array_element (Variables|Default|GetDynamicMaterialnsts)
        (Rendering|Material|SetScalarParameterValue _array_element "Fade" _fade :!class /Script/Engine.MaterialInstanceDynamic)))
    (:Finished
      (CallFunction|FadeFinishes _fade))))

(fn ConstructionScript
  (Utilities|Array|Clear (Variables|Default|GetDynamicMaterialnsts))
  (Variables|Default|SetOriginalMaterials (Rendering|Material|GetMaterials (Variables|Default|GetMesh)))
  (for _array_element (Variables|Default|GetFadeMaterialInsts)
    (bind _returnvalue (Rendering|Material|CreateDynamicMaterialInstance _array_element "None" "None" :!class /Script/Engine.KismetMaterialLibrary))
    (Utilities|Array|AddUnique (Variables|Default|GetDynamicMaterialnsts) _returnvalue)))

(fn SetMaterialtoDynamicInsts
  (for (_array_element _array_index) (Variables|Default|GetDynamicMaterialnsts)
    (Rendering|Material|SetMaterial (Variables|Default|GetMesh) _array_index _array_element)))

(fn ResetMaterials
  (for (_array_element _array_index) (Variables|Default|GetOriginalMaterials)
    (Rendering|Material|SetMaterial (Variables|Default|GetMesh) _array_index _array_element)))

(fn FadeFinishes
  (params (Fade :type Float%20%28single-precision%29))
  (if (>= Fade 1.0)
    (CallFunction|ResetMaterials)
    (elif (<= Fade 0.0)
      _)))
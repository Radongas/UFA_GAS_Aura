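; Enemy melee attack ability that turns the avatar toward its combat target and plays a random tagged attack montage.
; The montage's gameplay event triggers a small sphere search for live players at the montage's combat socket, damaging any non-friends found.
; A hit fires a melee impact gameplay cue carrying the montage tag, and the ability ends after that event or when the montage finishes or is interrupted.
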(event Ability|EventActivateAbility
  (bind _returnvalue (Ability|GetAvatarActorfromActorInfo))
  (bind _returnvalue_2 (Ability|GetAvatarActorfromActorInfo))
  (bind _returnvalue_3 (Ability|GetAvatarActorfromActorInfo))
  (Variables|Default|SetHasHitTarget false)
  (bind _returnvalue_4 (Class|EnemyInterface|GetCombatTarget(Message) _returnvalue))
  (bind _ascombat_interface (Utilities|Casting|CastToCombatInterface _returnvalue))
  (Class|CombatInterface|UpdateFacingTarget _ascombat_interface (Transformation|GetActorLocation _returnvalue_4))
  (bind _returnvalue_5 (Class|CombatInterface|GetAttackMontages(Message) _returnvalue))
  (bind _output_get (Variables|Default|SetTaggedMontage (Utilities|Array|Get(acopy) _returnvalue_5 (Math|Random|RandomIntegerinRange 0 (- (Utilities|Array|Length _returnvalue_5) 1)))))
  (if (> (Utilities|Array|Length _returnvalue_5) 0)
    (|PlayMontageandWaitProxy "None" (.Montage (Utilities|Struct|BreakTaggedMontage _output_get)) 1.0 "None" false 1.0 0.0 false
      (:then
        (Ability|Tasks|WaitGameplayEvent (.MontageTag (Utilities|Struct|BreakTaggedMontage _output_get)) 0
          (:EventReceived
            (bind _returnvalue_6 (Class|CombatInterface|GetCombatSocketLocation(Message) _returnvalue_2 (.SocketTag (Utilities|Struct|BreakTaggedMontage _output_get))))
            (bind _outoverlappingactors (Class|AuraAbilitySystemLibrary|GetLivePlayerWithinRadius _returnvalue_2 (Utilities|Array|MakeArray _returnvalue_2) 45.0 _returnvalue_6))
            (for _array_element _outoverlappingactors
              (if (Class|AuraAbilitySystemLibrary|IsNotFriend (Ability|GetAvatarActorfromActorInfo) _array_element)
                (Class|AuraDamageAbility|CauseDamage _array_element)
                (Variables|Default|SetHasHitTarget true)))
            (if (Variables|Default|GetHasHitTarget)
              (bind _returnvalue_7 (Class|EnemyInterface|GetCombatTarget(Message) _returnvalue_3))
              (Class|GameplayAbility|ExecuteGameplayCuewithParams "(TagName=\"GameplayCue.MeleeImpact\")" (Ability|GameplayCue|MakeGameplayCueParameters :AggregatedSourceTags (GameplayTags|MakeGameplayTagContainerfromTag (.montagetag (Variables|Default|GetTaggedMontage))) :Location _returnvalue_6 :EffectCauser _returnvalue_3 :SourceObject _returnvalue_7)))
            (Ability|EndAbility))))
      (:OnCompleted
        (Ability|EndAbility :!label _label))
      (:OnInterrupted
        (goto _label))
      (:OnCancelled
        (goto _label)))
    (else
      (Ability|EndAbility))))
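; Flame pillar actor Blueprint that makes its point light flicker like fire.
; From BeginPlay, it randomly picks one of two intensity timelines to play, scaling the curve by BaseIntensity to drive the light each update.
; When a timeline finishes, it picks again, so the flicker loops indefinitely with a varying sequence of the two patterns.
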(event Custom|StartTimeLine_2
  (bind _intensity (Timeline|FlameIntensityTimeLine_2 PlayFromStart)
    (:Update
      (Rendering|Components|Light|SetIntensity (Variables|Default|GetPointLight) (* _intensity (Variables|Default|GetBaseIntensity))))
    (:Finished
      (CallFunction|ChooseTimeLine))))

(event Custom|StartTimeLine_1
  (bind _intensity (Timeline|FlameIntensityTimeLine_1 PlayFromStart)
    (:Update
      (Rendering|Components|Light|SetIntensity (Variables|Default|GetPointLight) (* _intensity (Variables|Default|GetBaseIntensity))))
    (:Finished
      (CallFunction|ChooseTimeLine))))

(event Custom|ChooseTimeLine
  (switch int (Math|Random|RandomIntegerinRange 0 1)
    (:Default
      (CallFunction|StartTimeLine1 :!label _label))
    (:0
      (goto _label))
    (:1
      (CallFunction|StartTimeLine2))))

(event EventBeginPlay
  (CallFunction|ChooseTimeLine))

(fn ConstructionScript)